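; Tower turret Blueprint that aims at and shoots any actor entering its trigger volume.
; Overlap events store the target and toggle a lock flag, which Tick reads to choose between tracking and an idle yaw spin.
; Gun rotation is smoothed with RInterpTo, and the pitch clamp is left unconnected.
; While locked, a Delay called from Tick paces Projectile_BP spawns at the BarrelEnd socket.
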(event OnComponentBeginOverlap(TriggerVolume)
  (params (OverlappedComponent :type Primitive%20Component%20Object%20Reference) (OtherActor :type Actor%20Object%20Reference) (OtherComp :type Primitive%20Component%20Object%20Reference) (OtherBodyIndex :type Integer) (bFromSweep :type Boolean) (SweepResult :type Hit%20Result%20Structure%20%28by%20ref%29))
  ;[1 1 1] Quando o personagem entra na área, detecta o personagem e set a variável Targetlocket para true
  (Development|PrintString "In" true false)
  (Variables|Default|SetTarget OtherActor)
  (Variables|Default|SetTargetLocked? true))

(event OnComponentEndOverlap(TriggerVolume)
  (params (OverlappedComponent :type Primitive%20Component%20Object%20Reference) (OtherActor :type Actor%20Object%20Reference) (OtherComp :type Primitive%20Component%20Object%20Reference) (OtherBodyIndex :type Integer))
  ;[1 1 1] Quando o personagem sai da área a variável targetlocket é set para false
  (Development|PrintString "Out" true false)
  (Variables|Default|SetTargetLocked? false))

(event Custom|UpdateTurretRotation
  (bind _target (Variables|Default|GetTarget))
  (bind _tower1_gun (Variables|Default|GetTower1_Gun))
  (bind _returnvalue (Transformation|GetActorLocation _target))
  (bind _returnvalue_2 (Transformation|GetWorldLocation _tower1_gun))
  (bind _returnvalue_3 (Math|Rotator|FindLookatRotation _returnvalue_2 _returnvalue))
  (bind (_roll _pitch _yaw) (Math|Rotator|BreakRotator _returnvalue_3))
  ;[1 1 1] Faz a torret mirar no ator
  (Transformation|SetWorldRotation (Variables|Default|GetTower1_Gun) (Math|Interpolation|RInterpTo (Transformation|GetWorldRotation (Variables|Default|GetTower1_Gun)) (Math|Rotator|MakeRotator 0.0 _pitch _yaw) (Variables|Default|GetDeltaTime) 5.0) false false))

(event Custom|Idle
  (bind _tower1_gun (Variables|Default|GetTower1_Gun))
  (bind _returnvalue (Transformation|GetWorldRotation _tower1_gun))
  ;[1 1 1] Estado ocioso da torret
  (Transformation|SetWorldRotation (Variables|Default|GetTower1_Gun) (Math|Interpolation|RInterpTo _returnvalue (Math|Rotator|MakeRotator 0.0 0.0 (+ (.Yaw (Math|Rotator|BreakRotator _returnvalue)) 5.0)) (Variables|Default|GetDeltaTime) 5.0) false false))

(event Custom|FireTurret
  ;[1 1 1] Quando chamado evento de tiro, gerencia a cadência do disparo e spawna a bala
  (Utilities|FlowControl|Delay 0.6)
  (Game|SpawnActorfromClass "/Game/Assets/Projectile_BP.Projectile_BP_C" (Transformation|GetSocketTransform (Variables|Default|GetTower1_Gun) "BarrelEnd" "RTS_World") "Undefined" 0 0))

(event EventTick
  (params (DeltaSeconds :type Float%20%28single-precision%29))
  ;[1 1 1] Verifica se o alvo está na área
  (Variables|Default|SetDeltaTime DeltaSeconds)
  (if (Variables|Default|GetTargetLocked?)
    (CallFunction|UpdateTurretRotation)
    ;[1 1 1] Se estiver, chama evento de disparo
    (CallFunction|FireTurret)
    (else
      (CallFunction|Idle))))

(fn ConstructionScript)